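; Pressure plate actor that unlocks a linked Door when enough weight rests on it and locks it again when weight drops below the threshold.
; Overlap begin and end add or subtract the other actor's primitive component mass from a running TotalWeight, compared against ActivationWeight.
; An IsActivated flag ensures the activated and deactivated events fire only on state changes, with their handlers driving the Door.
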(event `Activated_Event`
  (`/Game/Blueprints/Puerta_BPxd.UnlockAuto_Event` (`self.Door`)))

(event `Deactivated_Event`
  (`/Game/Blueprints/Puerta_BPxd.Lock_Event` (`self.Door`)))

(event `self.ReceiveActorBeginOverlap`
  (params (OtherActor :type "Actor Object Reference"))
  (bind _output_get (set `self.TotalWeight` (+ (`PrimitiveComponent.GetMass` (`self.GetComponentByClass` OtherActor "/Script/Engine.PrimitiveComponent")) (`self.TotalWeight`))))
  (`/Engine/EditorBlueprintResources/StandardMacros.CompareFloat` _output_get (`self.ActivationWeight`)
    (:`>`
      _)
    (:`==`
      _))
  (if (not (`self.isActivated`))
    (set `self.isActivated` true)
    (`self.Activated_Event`)))

(event `self.ReceiveActorEndOverlap`
  (params (OtherActor :type "Actor Object Reference"))
  (bind _output_get (set `self.TotalWeight` (- (`self.TotalWeight`) (`PrimitiveComponent.GetMass` (`self.GetComponentByClass` OtherActor "/Script/Engine.PrimitiveComponent")))))
  (`/Engine/EditorBlueprintResources/StandardMacros.CompareFloat` _output_get (`self.ActivationWeight`)
    (:`<`
      (if (`self.isActivated`)
        (set `self.isActivated` false)
        (`self.Deactivated_Event`)))))

(fn `UserConstructionScript`)