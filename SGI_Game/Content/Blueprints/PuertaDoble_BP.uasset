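; PuertaDoble_BP is a double door actor that swings both leaves open when Open_Event is called.
; BeginPlay caches each mesh's world rotation as its closed pose.
; Open_Event plays a timeline whose two angle tracks drive a separate yaw offset for each leaf, combined with the cached rotation.
; It contains no trigger or closing logic.
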(event `self.ReceiveBeginPlay`
  (set `self.InitialRotation0` (`SceneComponent.K2_GetComponentRotation` (`self.StaticMeshComponent0`)))
  (set `self.InitialRotation1` (`SceneComponent.K2_GetComponentRotation` (`self.StaticMeshComponent01`))))

(event `Open_Event`
  (bind (_direction _openangle0 _openangle1) (`Timeline|Timeline_0`)
    (:`Update`
      (`SceneComponent.K2_SetWorldRotation` (`self.StaticMeshComponent0`) (`KismetMathLibrary.ComposeRotators` (`self.InitialRotation0`) (`KismetMathLibrary.MakeRotator` 0.0 0.0 _openangle0)) false false)
      (`SceneComponent.K2_SetWorldRotation` (`self.StaticMeshComponent01`) (`KismetMathLibrary.ComposeRotators` (`self.InitialRotation1`) (`KismetMathLibrary.MakeRotator` 0.0 0.0 _openangle1)) false false))))

(fn `UserConstructionScript`)