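; Keypad code manager actor that checks entered digits against a requested code to control a linked door.
; Button presses append digits to the entered code and trigger validation once the count reaches the code length.
; Validation compares each digit by index, then unlocks and opens the door with a success sound, or locks it with a fail sound.
; The entered digits and press count are cleared after every attempt.
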(event `CodeComplete_Event`
  (bind _returnvalue (`self.K2_GetActorLocation`))
  (bind _door (`self.Door`))
  (set `self.codeCorrect` true)
  (for (_array_element _array_index) (`self.CodeIntrodeced`)
    (`/Engine/EditorBlueprintResources/StandardMacros.CompareInt` _array_element (`|GetArrayItem` (`self.CodeRequested`) _array_index)
      (:`>`
        _)
      (:`<`
        _))
    (set `self.codeCorrect` false))
  (if (`self.codeCorrect`)
    (`/Game/Blueprints/Puerta_BPxd.Unlock_Event` _door)
    (`/Game/Blueprints/Puerta_BPxd.Open_Event` _door)
    (`GameplayStatics.PlaySoundAtLocation` "/Game/Sound/Success.Success" _returnvalue (struct) 1.0 1.0 0.0 null null null)
    (else
      (`/Game/Blueprints/Puerta_BPxd.Lock_Event` _door)
      (`GameplayStatics.PlaySoundAtLocation` "/Game/Sound/Fail.Fail" _returnvalue (struct) 1.0 1.0 0.0 null null null)))
  (`self.Reset_Event`))

(event `Reset_Event`
  (`KismetArrayLibrary.Array_Clear` (`self.CodeIntrodeced`))
  (set `self.ButtonsPressed` 0))

(event `ButtonPressed_Event`
  (params (digit :type Integer))
  (bind _buttonspressed (`self.ButtonsPressed`))
  (`/Engine/EditorBlueprintResources/StandardMacros.IncrementInt` _buttonspressed
    (:`  `
      (`KismetArrayLibrary.Array_Add` (`self.CodeIntrodeced`) digit)
      (`/Engine/EditorBlueprintResources/StandardMacros.CompareInt` _buttonspressed (`self.CodeLength`)
        (:`==`
          (`self.CodeComplete_Event`))))))

(fn `UserConstructionScript`)