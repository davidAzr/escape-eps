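; ColorPlate_BP is a plate that switches on while a KeyColorBox_BP of matching color overlaps it.
; Begin and end overlap events cast the other actor and compare its integer Color to the plate's own, setting Active true or false on a match.
; After either change, it calls CheckActivationEvent on its Manager reference, if valid.
; Active is a plain flag, so any matching box leaving clears it even if another remains.
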(event `self.ReceiveActorEndOverlap`
  (params (OtherActor :type "Actor Object Reference"))
  (bind _manager (`self.Manager`))
  (bind _askey_color_box_bp (cast `/Game/Blueprints/KeyColorBox_BP` OtherActor))
  (`/Engine/EditorBlueprintResources/StandardMacros.CompareInt` (`/Game/Blueprints/KeyColorBox_BP.color` _askey_color_box_bp) (`self.color`)
    (:`==`
      (set `self.Active` false)
      (if (`KismetSystemLibrary.IsValid` _manager) :!label _label
        (`/Game/Blueprints/ColorPlateManager.CheckActivation_Event` _manager)))))

(event `self.ReceiveActorBeginOverlap`
  (params (OtherActor :type "Actor Object Reference"))
  (bind _askey_color_box_bp (cast `/Game/Blueprints/KeyColorBox_BP` OtherActor))
  (`/Engine/EditorBlueprintResources/StandardMacros.CompareInt` (`/Game/Blueprints/KeyColorBox_BP.color` _askey_color_box_bp) (`self.color`)
    (:`==`
      (set `self.Active` true)
      (goto _label))))

(fn `UserConstructionScript`)