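; Trigger volume actor that lets the player open a linked door (Puerta) from within its bounds.
; Begin overlap shows the door's front and back hint messages and enables input on this actor; end overlap hides them and disables input.
; Pressing E or the gamepad bottom face button calls the door's OpenEvent if the player pawn is still overlapping.
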(event `Key|Gamepad_FaceButton_Bottom`
  (params (Key :type "Key Structure"))
  (:`Pressed`
    (if (`self.IsOverlappingActor` (`GameplayStatics.GetPlayerPawn` 0)) :!label _label
      (`/Game/Blueprints/Puerta_BPxd.Open_Event` (`self.Puerta`)))))

(event `Key|E`
  (params (Key :type "Key Structure"))
  (:`Pressed`
    (goto _label)))

(event `self.ReceiveActorBeginOverlap`
  (params (OtherActor :type "Actor Object Reference"))
  (bind _puerta (`self.Puerta`))
  (`SceneComponent.SetVisibility` (`/Game/Blueprints/Puerta_BPxd.HintMessage` _puerta) true false)
  (`SceneComponent.SetVisibility` (`/Game/Blueprints/Puerta_BPxd.HintMessage_Back` _puerta) true false)
  (`self.EnableInput` (`GameplayStatics.GetPlayerController` 0)))

(event `self.ReceiveActorEndOverlap`
  (params (OtherActor :type "Actor Object Reference"))
  (bind _puerta (`self.Puerta`))
  (`SceneComponent.SetVisibility` (`/Game/Blueprints/Puerta_BPxd.HintMessage` _puerta) false false)
  (`SceneComponent.SetVisibility` (`/Game/Blueprints/Puerta_BPxd.HintMessage_Back` _puerta) false false)
  (`self.DisableInput` (`GameplayStatics.GetPlayerController` 0)))

(fn `UserConstructionScript`)