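; Blinking light actor that makes its point light flicker briefly at random intervals.
; BeginPlay starts an endless delay loop that toggles visibility, toggles it back after a short fixed delay, then waits a random few seconds.
; Custom events control Hidden In Game separately: TurnOn_Event flips it, despite its name, while TurnOff_Event always hides the light.
; An unconnected random-chance flicker branch never runs.
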(event `self.ReceiveBeginPlay`
  (bind _pointlight (`self.PointLight`))
  (`SceneComponent.ToggleVisibility` _pointlight false :!label _label)
  (`KismetSystemLibrary.Delay` 0.2)
  (`SceneComponent.ToggleVisibility` _pointlight false)
  (`KismetSystemLibrary.Delay` (`KismetMathLibrary.RandomFloatInRange` 0.0 5.0))
  (goto _label))

(event `self.ReceiveTick`
  (params (DeltaSeconds :type "Float (single-precision)")))

(event `TurnOn_Event`
  (bind _pointlight (`self.PointLight`))
  (`SceneComponent.SetHiddenInGame` _pointlight (not (`SceneComponent.bHiddenInGame` _pointlight)) true))

(event `TurnOff_Event`
  (`SceneComponent.SetHiddenInGame` (`self.PointLight`) true false))

(fn `UserConstructionScript`)