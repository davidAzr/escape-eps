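; Door actor that can be locked, unlocked, opened and closed, with front and back text hints reflecting its state.
; Open_Event toggles the door, or first unlocks it if unlockable, while UnlockAuto_Event unlocks and opens it immediately.
; A timeline plays or reverses to swing yaw relative to the initial rotation, with a lock sound near the closed angle.
; Lock_Event reverses the timeline and locks, while Unlock_Event only marks the door unlockable.
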(event `UnlockAuto_Event`
  (bind _textclose (`self.TextClose`))
  (set `self.isUnlockable` false)
  (set `self.isLocked` false)
  (set `self.isClosed` false :!label _label)
  (`TextRenderComponent.K2_SetText` (`self.HintMessage`) _textclose)
  (`TextRenderComponent.K2_SetText` (`self.HintMessage_Back`) _textclose)
  (bind (_direction _openangle) (`Timeline|Timeline_0` :!label _label_2)
    (:`Update`
      (if (not (`self.SoundEmitted`))
        (`/Engine/EditorBlueprintResources/StandardMacros.CompareFloat` 0.1 _openangle
          (:`>`
            (`GameplayStatics.PlaySoundAtLocation` "/Game/Sound/door_lock.door_lock" (`self.K2_GetActorLocation`) (struct) 0.3 1.0 0.0 (`self.SoundAttenuation`) null null)
            (set `self.SoundEmitted` true))
          (:`==`
            _)
          (:`<`
            _)))
      (`self.K2_SetActorRotation` (`KismetMathLibrary.ComposeRotators` (`self.InitialRotation`) (`KismetMathLibrary.MakeRotator` 0.0 0.0 _openangle)))
      (if (`self.SoundEmitted`)
        (`KismetSystemLibrary.Delay` 0.2)
        (set `self.SoundEmitted` false)))))

(event `Lock_Event`
  (bind _textlocked (`self.TextLocked`))
  (set `self.isUnlockable` false)
  (set `self.isLocked` true)
  (`TextRenderComponent.K2_SetText` (`self.HintMessage`) _textlocked)
  (`TextRenderComponent.K2_SetText` (`self.HintMessage_Back`) _textlocked)
  (goto _label_2 :!via `Reverse`))

(event `Unlock_Event`
  (bind _textunlock (`self.TextUnlock`))
  (set `self.isUnlockable` true)
  (`TextRenderComponent.K2_SetText` (`self.HintMessage`) _textunlock)
  (`TextRenderComponent.K2_SetText` (`self.HintMessage_Back`) _textunlock))

(event `self.ReceiveBeginPlay`
  (bind _textlocked (`self.TextLocked`))
  (bind _textopen (`self.TextOpen`))
  (bind _hintmessage (`self.HintMessage`))
  (bind _hintmessage_back (`self.HintMessage_Back`))
  (bind _textunlock (`self.TextUnlock`))
  (set `self.InitialRotation` (`self.K2_GetActorRotation`))
  ;[1 1 1] Initial hint message setup
  (if (`self.isLocked`)
    (if (`self.isUnlockable`)
      (`TextRenderComponent.K2_SetText` _hintmessage _textunlock)
      (`TextRenderComponent.K2_SetText` _hintmessage_back _textunlock)
      (else
        (`TextRenderComponent.K2_SetText` _hintmessage _textlocked)
        (`TextRenderComponent.K2_SetText` _hintmessage_back _textlocked)))
    (else
      (`TextRenderComponent.K2_SetText` _hintmessage _textopen :!label _label_3)
      (`TextRenderComponent.K2_SetText` _hintmessage_back _textopen))))

(event `Open_Event`
  (bind _textlocked (`self.TextLocked`))
  (bind _hintmessage (`self.HintMessage`))
  (bind _textopen (`self.TextOpen`))
  (if (`self.isLocked`)
    (if (`self.isUnlockable`)
      (set `self.isUnlockable` false)
      (set `self.isLocked` false)
      (goto _label_3)
      (else
        (`TextRenderComponent.K2_SetText` _hintmessage _textlocked)
        (`TextRenderComponent.K2_SetText` _hintmessage _textlocked)))
    (elif (`self.isClosed`)
      (goto _label)
      (else
        (set `self.isClosed` true)
        (`TextRenderComponent.K2_SetText` _hintmessage _textopen)
        (`TextRenderComponent.K2_SetText` (`self.HintMessage_Back`) _textopen)
        (goto _label_2 :!via `Reverse`)))))

(fn `UserConstructionScript`)