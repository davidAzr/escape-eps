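; Player pawn that lets the player pick up keys and collectible Guses, press buttons and switches, and grab physics objects.
; Each action line-traces physics bodies along the view direction within Range, then uses a cast chain to dispatch by actor type with sounds.
; Tick moves the PhysicsHandle target in front of the view and shows a contextual hint widget for the looked-at object.
; A GusInfo widget counts found Guses.
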(event `PickUp_Event`
  (bind _guswidget (`self.gusWidget`))
  (bind (_outlocation _outrotation) (`self.GetActorEyesViewPoint` (`GameplayStatics.GetPlayerController` 0)))
  (bind (_outhit _returnvalue) (`KismetSystemLibrary.LineTraceSingleForObjects` _outlocation (+ (* (`KismetMathLibrary.GetForwardVector` _outrotation) (`self.range`)) _outlocation) (`|MakeArray` "ObjectTypeQuery4" :!type "EObjectTypeQuery Enum")))
  (if _returnvalue
    (bind (_bblockinghit _binitialoverlap _time _distance _location _impactpoint _normal _impactnormal _physmat _hitactor) (`GameplayStatics.BreakHitResult` _outhit))
    (bind _askey (cast `/Game/Blueprints/Key` _hitactor)
      (:`then`
        (`/Game/Blueprints/Key.PickUp_Event` _askey)
        (`GameplayStatics.PlaySound2D` "/Game/Sound/PickUp.PickUp" 1.0 1.0 0.0 null null))
      (:`CastFailed`
        (bind _asgus_bp (cast `/Game/Blueprints/Gus_BP` _hitactor)
          (:`then`
            (bind _output_get (set `/Game/UI/GusInfo.guses_found` (+ (`/Game/UI/GusInfo.guses_found` _guswidget) 1) _guswidget))
            (set `/Game/UI/GusInfo.text_guses` (`KismetTextLibrary.Conv_IntToText` _output_get) _guswidget)
            (`self.K2_DestroyActor` _asgus_bp)
            (`GameplayStatics.PlaySound2D` "/Game/Sound/PickUp.PickUp" 1.0 1.0 0.0 null null))
          (:`CastFailed`
            (bind _asbutton_bp (cast `/Game/Blueprints/Button_BP` _hitactor)
              (:`then`
                (`/Game/Blueprints/Button_BP.Press_Event` _asbutton_bp)
                (`GameplayStatics.PlaySound2D` "/Game/Sound/ButtonPressed.ButtonPressed" 1.0 1.0 0.0 null null))
              (:`CastFailed`
                (bind _aslight_switch (cast `/Game/Blueprints/LightSwitch` _hitactor)
                  (:`then`
                    (`/Game/Blueprints/LightSwitch.OnPressed_Event` _aslight_switch)
                    (`GameplayStatics.PlaySound2D` "/Game/Sound/LightSwitch.LightSwitch" 1.0 1.0 0.0 null null))
                  (:`CastFailed`
                    (bind _asdoors_button (cast `/Game/Blueprints/DoorsButton` _hitactor)
                      (:`then`
                        (`/Game/Blueprints/DoorsButton.OnPressed_Event` _asdoors_button)
                        (`GameplayStatics.PlaySound2D` "/Game/Sound/Button.Button" 1.0 1.0 0.0 null null))
                      (:`CastFailed`
                        (bind _aslights_button (cast `/Game/Blueprints/LightsButton` _hitactor))
                        (`/Game/Blueprints/LightsButton.OnPressed_Event` _aslights_button)
                        (`GameplayStatics.PlaySound2D` "/Game/Sound/Button.Button" 1.0 1.0 0.0 null null)))))))))))))

(event `self.ReceiveBeginPlay`
  (`self.EnableInput` (`GameplayStatics.GetPlayerController` 0))
  (bind _returnvalue (`|CreateWidget` "/Game/UI/GusInfo.GusInfo_C"))
  (set `self.gusWidget` _returnvalue)
  (`UserWidget.AddToViewport` _returnvalue 0)
  (bind _returnvalue_2 (`|CreateWidget` "/Game/UI/InformativeMessage.InformativeMessage_C"))
  (set `self.Informative` _returnvalue_2))

(event `Key|E`
  (params (Key :type "Key Structure"))
  (:`Pressed`
    (`self.PickUp_Event` :!label _label)))

(event `Key|Gamepad_FaceButton_Bottom`
  (params (Key :type "Key Structure"))
  (:`Pressed`
    (goto _label)))

(event `Key|LeftMouseButton`
  (params (Key :type "Key Structure"))
  (:`Pressed`
    (`self.Grab_Event` :!label _label_2))
  (:`Released`
    (`self.Drop_Event` :!label _label_3)))

(event `Key|Gamepad_RightShoulder`
  (params (Key :type "Key Structure"))
  (:`Pressed`
    (goto _label_2))
  (:`Released`
    (goto _label_3)))

(event `Grab_Event`
  (bind (_outlocation _outrotation) (`self.GetActorEyesViewPoint` (`GameplayStatics.GetPlayerController` 0)))
  (bind (_outhit _returnvalue) (`KismetSystemLibrary.LineTraceSingleForObjects` _outlocation (+ (* (`KismetMathLibrary.GetForwardVector` _outrotation) (`self.range`)) _outlocation) (`|MakeArray` "ObjectTypeQuery4" :!type "EObjectTypeQuery Enum")))
  (if _returnvalue
    (bind (_bblockinghit _binitialoverlap _time _distance _location _impactpoint _normal _impactnormal _physmat _hitactor _hitcomponent) (`GameplayStatics.BreakHitResult` _outhit))
    (cast `/Game/Blueprints/Button_BP` _hitactor
      (:`CastFailed`
        (`PhysicsHandleComponent.GrabComponentAtLocationWithRotation` (`self.PhysicsHandle`) _hitcomponent "None" _location (`KismetMathLibrary.MakeRotator` 0.0 0.0 (.yaw (`.OutRotation` (`self.GetActorEyesViewPoint` (`GameplayStatics.GetPlayerController` 0))))))))))

(event `Drop_Event`
  (`PhysicsHandleComponent.ReleaseComponent` (`self.PhysicsHandle`)))

(event `self.ReceiveTick`
  (params (DeltaSeconds :type "Float (single-precision)"))
  (bind _informative (`self.Informative`))
  (bind _islookingobject (`self.isLookingObject`))
  (bind _informative_2 (`self.Informative`))
  (bind _informative_3 (`self.Informative`))
  (bind _informative_4 (`self.Informative`))
  (bind _informative_5 (`self.Informative`))
  (bind _informative_6 (`self.Informative`))
  (bind (_outlocation _outrotation) (`self.GetActorEyesViewPoint` (`GameplayStatics.GetPlayerController` 0)))
  (bind (_outlocation_2 _outrotation_2) (`self.GetActorEyesViewPoint` (`GameplayStatics.GetPlayerController` 0)))
  (`PhysicsHandleComponent.SetTargetLocationAndRotation` (`self.PhysicsHandle`) (+ (* (`KismetMathLibrary.GetForwardVector` _outrotation_2) (`self.range`)) _outlocation_2) (`KismetMathLibrary.MakeRotator` 0.0 0.0 (.yaw (`.OutRotation` (`self.GetActorEyesViewPoint` (`GameplayStatics.GetPlayerController` 0))))))
  (bind (_outhit _returnvalue) (`KismetSystemLibrary.LineTraceSingleForObjects` _outlocation (+ (* (`KismetMathLibrary.GetForwardVector` _outrotation) (`self.range`)) _outlocation) (`|MakeArray` "ObjectTypeQuery4" :!type "EObjectTypeQuery Enum")))
  (if _returnvalue
    (bind (_bblockinghit _binitialoverlap _time _distance _location _impactpoint _normal _impactnormal _physmat _hitactor) (`GameplayStatics.BreakHitResult` _outhit))
    (bind _askey (cast `/Game/Blueprints/Key` _hitactor)
      (:`then`
        (set `/Game/UI/InformativeMessage.textToDisplay` (`/Game/Blueprints/Key.description` _askey) _informative_6)
        (if (not _islookingobject)
          (`UserWidget.AddToViewport` _informative_6 0)
          (set `self.isLookingObject` true :!label _label_4)))
      (:`CastFailed`
        (bind _asgus_bp (cast `/Game/Blueprints/Gus_BP` _hitactor)
          (:`then`
            (set `/Game/UI/InformativeMessage.textToDisplay` (`/Game/Blueprints/Gus_BP.Name` _asgus_bp) _informative_3)
            (if (not _islookingobject)
              (`UserWidget.AddToViewport` _informative_3 0)
              (goto _label_4)))
          (:`CastFailed`
            (cast `/Game/Blueprints/Button_BP` _hitactor
              (:`then`
                (set `/Game/UI/InformativeMessage.textToDisplay` "Press" _informative_5)
                (if (not _islookingobject)
                  (`UserWidget.AddToViewport` _informative_5 0)
                  (goto _label_4)))
              (:`CastFailed`
                (bind _aslight_switch (cast `/Game/Blueprints/LightSwitch` _hitactor)
                  (:`then`
                    (set `/Game/UI/InformativeMessage.textToDisplay` (`KismetTextLibrary.Conv_TextToString` (`/Game/Blueprints/LightSwitch.TextToDisplay` _aslight_switch)) _informative)
                    (if (not _islookingobject)
                      (`UserWidget.AddToViewport` _informative 0)
                      (goto _label_4)))
                  (:`CastFailed`
                    (bind _asdoors_button (cast `/Game/Blueprints/DoorsButton` _hitactor)
                      (:`then`
                        (set `/Game/UI/InformativeMessage.textToDisplay` (`KismetTextLibrary.Conv_TextToString` (`/Game/Blueprints/DoorsButton.TextToDisplay` _asdoors_button)) _informative_2)
                        (if (not _islookingobject)
                          (`UserWidget.AddToViewport` _informative_2 0)
                          (goto _label_4)))
                      (:`CastFailed`
                        (bind _aslights_button (cast `/Game/Blueprints/LightsButton` _hitactor))
                        (set `/Game/UI/InformativeMessage.textToDisplay` (`KismetTextLibrary.Conv_TextToString` (`/Game/Blueprints/LightsButton.TextToDisplay` _aslights_button)) _informative_4)
                        (if (not _islookingobject)
                          (`UserWidget.AddToViewport` _informative_4 0)
                          (goto _label_4))))))))))))
    (elif (`self.isLookingObject`)
      (`Widget.RemoveFromParent` _informative_6)
      (set `self.isLookingObject` false))))

(fn `UserConstructionScript`)