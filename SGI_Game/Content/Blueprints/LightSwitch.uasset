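; Light switch actor that controls an array of lights and maintains a text prompt built from an action and a description.
; While enabled, each press calls TurnOnEvent on every light, whatever the current action, and flips the label between "Turn on" and "Turn off".
; Disabling turns all lights off, so later presses only report a broken switch.
; Re-enabling restores the prompt without resetting the action.
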(event `self.ReceiveBeginPlay`
  (set `self.TextToDisplay` (`KismetTextLibrary.Conv_StringToText` (`KismetStringLibrary.Concat_StrStr` (`self.Action`) (`self.Description`)))))

(event `Disable_Event`
  (set `self.enabled` false)
  (for _array_element (`self.Lights`)
    (`/Game/Blueprints/BlinkingLight.TurnOff_Event` _array_element)))

(event `Enable_Event`
  (set `self.TextToDisplay` (`KismetTextLibrary.Conv_StringToText` (`KismetStringLibrary.Concat_StrStr` (`self.Action`) (`self.Description`))))
  (set `self.enabled` true))

(event `OnPressed_Event`
  (if (`self.enabled`)
    (for _array_element (`self.Lights`)
      (`/Game/Blueprints/BlinkingLight.TurnOn_Event` _array_element))
    (if (`KismetStringLibrary.EqualEqual_StrStr` (`self.Action`) "Turn on ")
      (set `self.Action` "Turn off ")
      (else
        (set `self.Action` "Turn on ")))
    (set `self.TextToDisplay` (`KismetTextLibrary.Conv_StringToText` (`KismetStringLibrary.Concat_StrStr` (`self.Action`) (`self.Description`))))
    (else
      (set `self.TextToDisplay` "The switch is not working"))))

(fn `UserConstructionScript`)