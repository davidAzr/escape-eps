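; LightsButton is a pressable button Blueprint that toggles a group of linked switches on and off.
; Each press calls EnableEvent or DisableEvent on every entry in Switches according to the Locked flag, then flips that flag.
; The construction script creates a dynamic red material on the button mesh, whose Intensidad vector turns bright when enabling and dim when disabling.
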(event `OnPressed_Event`
  (bind _locked (`self.Locked`))
  (bind _material (`self.material`))
  (for _array_element (`self.Switches`)
    (if _locked
      (`/Game/Blueprints/LightSwitch.Enable_Event` _array_element)
      (`MaterialInstanceDynamic.SetVectorParameterValue` _material "Intensidad" (struct :`R` 1.0 :`A` 1.0))
      (else
        (`/Game/Blueprints/LightSwitch.Disable_Event` _array_element)
        (`MaterialInstanceDynamic.SetVectorParameterValue` _material "Intensidad" (struct :`R` 0.3 :`A` 1.0)))))
  (set `self.Locked` (not _locked)))

(fn `UserConstructionScript`
  (bind _returnvalue (`PrimitiveComponent.CreateDynamicMaterialInstance` (`self.Button`) 1 "/Game/Props/Boton/rojo.rojo" "None"))
  (set `self.Material` _returnvalue))